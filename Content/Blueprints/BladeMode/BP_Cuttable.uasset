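; Cuttable actor for Blade Mode that can be sliced along an arbitrary plane at runtime.
; The construction script copies the assigned static mesh into a procedural mesh with collision, then destroys the static mesh component.
; Slice cuts a given procedural mesh by location and normal, caps the cut with a supplied material and enables physics on the newly created half.
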(event `self.ReceiveBeginPlay`)

(fn `Slice`
  (params (ProceduralMesh :type "ProceduralMeshComponent Object Reference") (Location :type "Vector Structure") (Normal :type "Vector Structure") (CapMaterial :type "Material Object Reference"))
  (bind _outotherhalfprocmesh (`KismetProceduralMeshLibrary.SliceProceduralMesh` ProceduralMesh Location Normal true "CreateNewSectionForCap" CapMaterial))
  (`PrimitiveComponent.SetSimulatePhysics` _outotherhalfprocmesh true))

(fn `UserConstructionScript`
  (`StaticMeshComponent.SetStaticMesh` (`self.StaticMesh`) (`self.MeshToCopy`))
  (`KismetProceduralMeshLibrary.CopyProceduralMeshFromStaticMeshComponent` (`self.StaticMesh`) 0 (`self.ProceduralMesh`) true)
  (`ActorComponent.K2_DestroyComponent` (`self.StaticMesh`)))