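; BP_PlaneCutter is a player-controlled blade-mode pawn that moves and rotates a translucent plane to slice procedural meshes.
; Axis inputs drive swept movement and plane roll, while Tick tints the plane yellow when overlapping BP_Cuttable actors and red otherwise.
; Jump slices overlapping ProceduralMeshComponents along the plane with a glowing cap, enables physics on the new half and pushes both halves apart with opposing impulses.
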(event `self.ReceiveBeginPlay`
  (bind _returnvalue (`PrimitiveComponent.CreateDynamicMaterialInstance` (`self.Plane`) 0 "/Game/Material/M_TranslucentPlane.M_TranslucentPlane" "None"))
  (set `self.Material` _returnvalue))

(event `self.ReceiveTick`
  (params (DeltaSeconds :type "Float (single-precision)"))
  (bind _material (`self.Material`))
  ;[1 1 1] Consume Movement
  (bind _returnvalue (`self.ConsumeMovementInputVector`))
  (`self.K2_AddActorLocalOffset` (* _returnvalue DeltaSeconds) true)
  ;[1 1 1] Process Cuttable
  (if (== (`KismetArrayLibrary.Array_Length` (`PrimitiveComponent.GetOverlappingActors` (`self.Plane`) "/Game/Blueprints/BladeMode/BP_Cuttable.BP_Cuttable_C")) 0)
    (`MaterialInstanceDynamic.SetVectorParameterValue` _material "Color" (struct :`R` 1.0 :`A` 1.0))
    (else
      (`MaterialInstanceDynamic.SetVectorParameterValue` _material "Color" (struct :`R` 1.0 :`G` 1.0 :`A` 1.0)))))

(event `InputAction|Jump`
  (params (Key :type "Key Structure"))
  (bind _plane (`self.Plane`))
  (bind _outoverlappingcomponents (`PrimitiveComponent.GetOverlappingComponents` (`self.Plane`)))
  ;[1 1 1] Cut
  (:`Pressed`
    (if (not (== (`KismetArrayLibrary.Array_Length` _outoverlappingcomponents) 0))
      (for _array_element _outoverlappingcomponents
        (bind _asprocedural_mesh_component (cast `ProceduralMeshComponent` _array_element))
        (`KismetSystemLibrary.PrintString` "Cut Successful")
        (`self.SliceProceduralMesh` _asprocedural_mesh_component (`SceneComponent.K2_GetComponentLocation` _plane) (`SceneComponent.GetUpVector` _plane) "/Game/Material/M_Glow.M_Glow")))))

(event `InputAxis|Forward`
  (params (AxisValue :type "Float (single-precision)"))
  ;[1 1 1] Movement
  (`self.AddMovementInput` (`self.GetActorForwardVector`) (* AxisValue (`self.MaxSpeed`))))

(event `InputAxis|Right`
  (params (AxisValue :type "Float (single-precision)"))
  ;[1 1 1] Movement
  (`self.AddMovementInput` (`self.GetActorRightVector`) (* AxisValue (`self.MaxSpeed`))))

(event `InputAxis|RotateLeft`
  (params (AxisValue :type "Float (single-precision)"))
  ;[1 1 1] Movement
  (bind _output_get (set `self.PlaneRotation` (+ AxisValue (`self.PlaneRotation`))))
  (`SceneComponent.K2_SetRelativeRotation` (`self.Plane`) (`KismetMathLibrary.MakeRotator` _output_get 90.0) false false))

(fn `SliceProceduralMesh`
  (params (ProceduralMesh :type "ProceduralMeshComponent Object Reference") (Location :type "Vector Structure") (Normal :type "Vector Structure") (CapMaterial :type "Material Object Reference"))
  (bind _outotherhalfprocmesh (`KismetProceduralMeshLibrary.SliceProceduralMesh` ProceduralMesh Location Normal true "CreateNewSectionForCap" CapMaterial))
  (`PrimitiveComponent.SetSimulatePhysics` _outotherhalfprocmesh true)
  (`PrimitiveComponent.AddImpulse` _outotherhalfprocmesh (* Normal 10) "None" true)
  (`PrimitiveComponent.AddImpulse` ProceduralMesh (* Normal -10) "None" true))

(fn `UserConstructionScript`)